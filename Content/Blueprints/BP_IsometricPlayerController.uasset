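; Player controller for an isometric, grid-based tower placement game, handling camera input, cursor, menu and tower placement.
; On BeginPlay it adds input mappings, views through the level's IsometricCamera, creates a hidden HUD and caches the GridManager.
; Rotate and zoom inputs feed the camera, while the menu key toggles the HUD and player input context.
; Each tick snaps the ghost tower to the cell under the cursor; placing passes the cursor hit to GridManager.
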(event `self.ReceiveBeginPlay`
  (bind _returnvalue (`GameplayStatics.GetPlayerController` 0))
  (bind _returnvalue_2 (pcsubsystem `EnhancedInputLocalPlayerSubsystem` _returnvalue))
  (`EnhancedInputSubsystemInterface.AddMappingContext` _returnvalue_2 "/Game/Input/IMC_Player.IMC_Player" 1 (struct))
  (`EnhancedInputSubsystemInterface.AddMappingContext` _returnvalue_2 "/Game/Input/IMC_Global.IMC_Global" 0 (struct))
  (bind _outactors (`GameplayStatics.GetAllActorsOfClass` "/Script/Echoes.IsometricCamera"))
  (bind _output_get (set `self.Cam` (`|GetArrayItem` _outactors)))
  (`self.SetViewTargetWithBlend` _returnvalue _output_get 0.0 "VTBlend_Linear" 0.0 false)
  (set `self.bShowMouseCursor` true)
  (set `self.bEnableClickEvents` true)
  (set `self.bEnableMouseOverEvents` true)
  (bind _returnvalue_3 (`|CreateWidget` "/Game/Blueprints/WB_HUD.WB_HUD_C"))
  (bind _output_get_2 (set `self.HUD` _returnvalue_3))
  (`UserWidget.AddToViewport` _output_get_2 0)
  (`Widget.SetVisibility` (`self.HUD`) "Hidden")
  (bind _outactors_2 (`GameplayStatics.GetAllActorsOfClass` "/Script/Echoes.GridManager"))
  (set `self.GridManager` (`|GetArrayItem` _outactors_2)))

(event `self.ReceiveTick`
  (params (DeltaSeconds :type "Float (single-precision)"))
  (`self.MoveGhostTower`))

(event `EnhancedInput|/Game/Input/IA_RotateCamera`
  (params (ActionValue :type "Float (double-precision)") (ElapsedSeconds :type "Float (double-precision)") (TriggeredSeconds :type "Float (double-precision)") (InputAction :type "InputAction Object Reference" :default "/Game/Input/IA_RotateCamera.IA_RotateCamera"))
  ; Camera Control
  (:`Triggered`
    (`IsometricCamera.AddOrbitInput` (`self.Cam`) ActionValue)))

(event `EnhancedInput|/Game/Input/IA_ZoomCamera`
  (params (ActionValue :type "Float (double-precision)") (ElapsedSeconds :type "Float (double-precision)") (TriggeredSeconds :type "Float (double-precision)") (InputAction :type "InputAction Object Reference" :default "/Game/Input/IA_ZoomCamera.IA_ZoomCamera"))
  ; Camera Control
  (:`Triggered`
    (`IsometricCamera.AddZoomInput` (`self.Cam`) ActionValue)))

(event `EnhancedInput|/Game/Input/IA_OpenMenu`
  (params (ActionValue :type Boolean) (ElapsedSeconds :type "Float (double-precision)") (TriggeredSeconds :type "Float (double-precision)") (InputAction :type "InputAction Object Reference" :default "/Game/Input/IA_OpenMenu.IA_OpenMenu"))
  (bind _hud (`self.HUD`))
  (bind _returnvalue (not (`self.IsMenuVisible`)))
  (bind _returnvalue_2 (pcsubsystem `EnhancedInputLocalPlayerSubsystem` self))
  ; Handle Menu
  (:`Started`
    (if _returnvalue
      (`Widget.SetVisibility` _hud "Visible")
      (`EnhancedInputSubsystemInterface.RemoveMappingContext` _returnvalue_2 "/Game/Input/IMC_Player.IMC_Player" (struct))
      (else
        (`Widget.SetVisibility` _hud "Hidden")
        (`EnhancedInputSubsystemInterface.AddMappingContext` _returnvalue_2 "/Game/Input/IMC_Player.IMC_Player" 0 (struct))))
    (set `self.IsMenuVisible` _returnvalue)))

(event `EnhancedInput|/Game/Input/IA_PlaceTower`
  (params (ActionValue :type Boolean) (ElapsedSeconds :type "Float (double-precision)") (TriggeredSeconds :type "Float (double-precision)") (InputAction :type "InputAction Object Reference" :default "/Game/Input/IA_PlaceTower.IA_PlaceTower"))
  ; Place Tower
  (:`Started`
    (`GridManager.PlaceTower` (`self.GridManager`) (`.Location` (`GameplayStatics.BreakHitResult` (`self.GetHitResultUnderCursorByChannel` "TraceTypeQuery1"))))))

(fn `MoveGhostTower`
  (bind _gridmanager (`self.GridManager`))
  (bind _cellsize (`GridManager.CellSize` _gridmanager))
  (bind _ghosttowerinstance (`GridManager.GhostTowerInstance` (`self.GridManager`)))
  (bind _returnvalue (/ _cellsize 2.0))
  (bind (_row _column) (break `GridCell` (`GridManager.GetCellAtWorldPosition` _gridmanager (`.Location` (`GameplayStatics.BreakHitResult` (`self.GetHitResultUnderCursorByChannel` "TraceTypeQuery1"))))))
  (if (`KismetSystemLibrary.IsValid` _ghosttowerinstance)
    (`self.K2_SetActorLocation` _ghosttowerinstance (`KismetMathLibrary.MakeVector` (+ _returnvalue (* _column _cellsize)) (+ (* _row _cellsize) _returnvalue)) false false)))

(fn `UserConstructionScript`)