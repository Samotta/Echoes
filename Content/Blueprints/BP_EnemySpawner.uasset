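; Enemy spawner actor that periodically spawns StandardEnemy actors at the grid's start point.
; On BeginPlay it finds the GridManager, moves itself to that StartPoint and starts a looping timer using SpawnTimeInterval.
; Each timer tick runs SpawnEnemy, which always spawns at the spawner's location and rotation, with one added to each axis of its scale.
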(event `self.ReceiveBeginPlay`
  (bind _returnvalue (`GameplayStatics.GetActorOfClass` "/Script/Echoes.GridManager"))
  (bind _output_get (set `self.GridManager` _returnvalue))
  (`self.K2_SetActorLocation` (`GridManager.StartPoint` _output_get))
  (`KismetSystemLibrary.K2_SetTimer` null "SpawnEnemy" (`self.SpawnTimeInterval`) true))

(fn `SpawnEnemy`
  (bind (_returnvalue_location _returnvalue_rotation _returnvalue_scale) (`KismetMathLibrary.BreakTransform` (`self.GetTransform` self)))
  (`|SpawnActorFromClass` "/Game/Blueprints/StandardEnemy.StandardEnemy_C" (`KismetMathLibrary.MakeTransform` _returnvalue_location _returnvalue_rotation (+ _returnvalue_scale (1.0 1.0 1.0))) "AlwaysSpawn" "MultiplyWithRoot" null null))

(fn `UserConstructionScript`)